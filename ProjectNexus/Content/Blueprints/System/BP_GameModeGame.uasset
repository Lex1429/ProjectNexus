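; BP_GameModeGame is the gameplay game mode that spawns the selected character and shows the combat HUD.
; On BeginPlay it creates WBP_CombatUI for the first player controller and adds it to the viewport.
; Its GetDefaultPawnClassForController override uses the character class from the Game Instance's GetSelectedCharacterMessage, falling back to the parent's default pawn class when that class is invalid.
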(event EventBeginPlay
  (bind _returnvalue (UserInterface|CreateWidget "/Game/UI/WBP_CombatUI.WBP_CombatUI_C" (Game|GetPlayerController 0)))
  (UserInterface|Viewport|AddtoViewport _returnvalue 0))

(fn ConstructionScript)

(fn GetDefaultPawnClassforController
  (params (InController :type Controller%20Object%20Reference))
  (bind _returnvalue (|CallParentFunction InController))
  (bind _selectedcharacterclass (Class|BPIMissionSetup|GetSelectedCharacter(Message) (Game|GetGameInstance)))
  (if (Utilities|IsValidClass _selectedcharacterclass)
    (return _selectedcharacterclass)
    (else
      (return _returnvalue))))