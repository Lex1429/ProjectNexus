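; BP_MissionSetupGameMode is a game mode that spawns players as the character selected in the game instance.
; Its GetDefaultPawnClassForController override reads that class through GetSelectedCharacterMessage and falls back to the parent's default when the class is invalid.
; BeginPlay is empty; the nodes that create the mission select widget and set UI-only input are disconnected and never run.
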(event EventBeginPlay)

(fn ConstructionScript)

(fn GetDefaultPawnClassforController
  (params (InController :type Controller%20Object%20Reference))
  (bind _returnvalue (|CallParentFunction InController))
  (bind _selectedcharacterclass (Class|BPIMissionSetup|GetSelectedCharacter(Message) (Game|GetGameInstance)))
  (if (Utilities|IsValidClass _selectedcharacterclass)
    (return _selectedcharacterclass)
    (else
      (return _returnvalue))))