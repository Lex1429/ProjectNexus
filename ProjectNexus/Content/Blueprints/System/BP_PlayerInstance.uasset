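; BP_PlayerInstance stores player state for the game: maximum and current health plus the character class selected for mission levels.
; SetPlayerHealth and SetSelectedCharacter events receive messages and write those values into its variables.
; GetPlayerHealth and GetSelectedCharacter return the stored values to callers, with no other logic.
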(event EventSetSelectedCharacter
  (params (SelectedCharacterClass :type Pawn%20Class%20Reference))
  ;[1 1 1] Receives Message of Selected Character to use in Mission Levels
  (Variables|Default|SetSelectedCharacter SelectedCharacterClass))

(event EventSetPlayerHealth
  (params (MaxHealth :type Float%20%28double-precision%29) (CurrentHealth :type Float%20%28double-precision%29))
  ;[1 1 1] Receives Message of Player Health and Stores values
  (Variables|Default|SetMaxHealth MaxHealth)
  (Variables|Default|SetCurrentHealth CurrentHealth))

(fn GetPlayerHealth
  (return (Variables|Default|GetMaxHealth) (Variables|Default|GetCurrentHealth)))

(fn GetSelectedCharacter
  (return (Variables|Default|GetSelectedCharacter)))