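; Base player character that handles movement, health, XP leveling and passive upgrades, exposing its state through interface getters and setters.
; XP gains raise the level and open a paused level-up menu; passives boost max HP, fire rate or XP gain, with gameplay tags tracking three icon slots.
; Damage leads to a death sequence returning to MissionSetUp, and capsule overlaps trigger interactions.
; Active-ability triggers, trace attack and TakeDamage/Heal logic are unwired or empty.
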(event OnComponentBeginOverlap(CapsuleComponent)
  (params (OverlappedComponent :type Primitive%20Component%20Object%20Reference) (OtherActor :type Actor%20Object%20Reference) (OtherComp :type Primitive%20Component%20Object%20Reference) (OtherBodyIndex :type Integer) (bFromSweep :type Boolean) (SweepResult :type Hit%20Result%20Structure%20%28by%20ref%29))
  (bind _array_element (Utilities|Array|ForEachLoopwithBreak (Collision|GetOverlappingActors "/Script/Engine.Actor" :!class /Script/Engine.Actor) :!label _label)
    (:LoopBody
      (if (Utilities|DoesObjectImplementInterface _array_element "/Game/Blueprints/Interfaces/BPI_Interactions.BPI_Interactions_C")
        (GameplayTags|AddGameplayTag (Variables|Default|GetPlayerStateTag) "(TagName=\"Interacting\")" :!class /Script/GameplayTags.BlueprintGameplayTagLibrary)
        (Class|BPIInteractions|Interact(Message) _array_element)
        (goto _label Break)))))

(event OnComponentEndOverlap(CapsuleComponent)
  (params (OverlappedComponent :type Primitive%20Component%20Object%20Reference) (OtherActor :type Actor%20Object%20Reference) (OtherComp :type Primitive%20Component%20Object%20Reference) (OtherBodyIndex :type Integer))
  (GameplayTags|RemoveGameplayTag (Variables|Default|GetPlayerStateTag) "(TagName=\"Interacting\")" :!class /Script/GameplayTags.BlueprintGameplayTagLibrary))

(event Custom|OrbXPIncrease
  (params (IncomingXP :type Float%20%28double-precision%29))
  ;[1 1 1] Communicates with the XP orb to increase player XP
  (CallFunction|AddXp IncomingXP))

(event Custom|Death
  ;[1 1 1] Handles death sequence
  (Development|PrintString "Dead")
  (Components|Animation|PlayAnimation (Variables|Character|GetMesh) "/Game/Animations/TempAnimations2/Dying_Anim_mixamo_com.Dying_Anim_mixamo_com" false)
  (Input|DisableInput (Game|GetPlayerController 0))
  (Utilities|FlowControl|Delay 3.0)
  (Class|BPIMissionSetup|SetSelectedCharacter(Message) (Game|GetGameInstance) 0 "None")
  (Game|OpenLevel(byName) "MissionSetUp"))

(event Custom|DamageResponse
  (params (DamageResponse :type E_DamageResponse%20Enum :default "NewEnumerator0"))
  ;[1 1 1] TEMP | Damage type print
  (Development|PrintString (Utilities|String|EnumtoString DamageResponse)))

(event Custom|MaxHPPassive
  ;[1 1 1] Passive Ability Events
  (Passives|IncreaseMaxHP))

(event Custom|FireRatePassive
  ;[1 1 1] Passive Ability Events
  (Passives|IncreaseFireRate))

(event Custom|XPIncreasePassive
  ;[1 1 1] Passive Ability Events
  (Passives|IncreaseXPGain))

(event EventSetPlayerXP
  (params (CurrentXP :type Float%20%28double-precision%29))
  ;[1 1 1] Interface Dispatchers
  (Variables|Stats|SetCurrentXP CurrentXP))

(event EventSetXptoLevel
  (params (XpToLevel :type Float%20%28double-precision%29))
  ;[1 1 1] Interface Dispatchers
  (Variables|Stats|SetXPtoLevel XpToLevel))

(event EventSetPassive3
  (params (Passive3 :type Texture%202D%20Object%20Reference) (PassiveName :type Name :default "None"))
  ;[1 1 1] Passive Ability Interface Dispatchers
  (Variables|PassiveLevels|SetPassiveIcon3 Passive3)
  (Variables|PassiveLevels|SetPassiveName3 PassiveName))

(event Game|Damage|EventAnyDamage
  (params (Damage :type Float%20%28single-precision%29) (DamageType :type Damage%20Type%20Object%20Reference) (InstigatedBy :type Controller%20Object%20Reference) (DamageCauser :type Actor%20Object%20Reference))
  (bind _output_get (Variables|Stats|SetCurrentHealth (- (Variables|Stats|GetCurrentHealth) Damage)))
  (if (<= _output_get 0.0)
    (Utilities|FlowControl|DoOnce false
      (:Completed
        (Variables|Default|SetIsDead? true)
        (CallFunction|Death)))))

(event EventSetPlayerCurrentHealth
  (params (CurrentHealth :type Float%20%28double-precision%29))
  ;[1 1 1] Interface Dispatchers
  (Variables|Stats|SetCurrentHealth CurrentHealth))

(event EventSetPlayerLevel
  (params (PlayerLevel :type Integer))
  ;[1 1 1] Interface Dispatchers
  (Variables|Stats|SetPlayerLevel PlayerLevel))

(event EventSetAbilityTag
  (params (AbilityTag :type Gameplay%20Tag%20Container%20Structure))
  ;[1 1 1] Interface Dispatchers
  (Variables|Default|SetAbilitiesTag AbilityTag))

(event EventSetPlayerMaxHealth
  (params (MaxHealth :type Float%20%28double-precision%29))
  ;[1 1 1] Interface Dispatchers
  (Variables|Stats|SetMaxHealth MaxHealth))

(event EventSetMaxHPPassiveLvl
  (params (MaxHPLvl :type Integer))
  ;[1 1 1] Passive Ability Interface Dispatchers
  (Variables|PassiveLevels|SetMaxHPLevel MaxHPLvl))

(event EventTick
  (params (DeltaSeconds :type Float%20%28single-precision%29)))

(event EventSetAbility
  (params (PassiveAbility :type Data%20Table%20Object%20Reference))
  ;[1 1 1] Interface Dispatchers
  (Variables|Default|SetAssignedAbility PassiveAbility))

(event EventSetPassive1
  (params (Passive1 :type Texture%202D%20Object%20Reference) (PassiveName :type Name :default "None"))
  ;[1 1 1] Passive Ability Interface Dispatchers
  (Variables|PassiveLevels|SetPassiveIcon1 Passive1)
  (Variables|PassiveLevels|SetPassiveName1 PassiveName))

(event EventSetPassive2
  (params (Passive2 :type Texture%202D%20Object%20Reference) (PassiveName :type Name :default "None"))
  ;[1 1 1] Passive Ability Interface Dispatchers
  (Variables|PassiveLevels|SetPassiveIcon2 Passive2)
  (Variables|PassiveLevels|SetPassiveName2 PassiveName))

(event Input|AxisEvents|InputAxisForward/BackwardMovement
  (params (AxisValue :type Float%20%28single-precision%29))
  ;[1 1 1] Forward/Backward Movement.
  (Pawn|Input|AddMovementInput (Math|Vector|GetForwardVector (Math|Rotator|MakeRotator 0.0 0.0 (.yaw (Pawn|GetControlRotation :!class /Script/Engine.Pawn)))) AxisValue false))

(event Input|AxisEvents|InputAxisLeft/RightMovement
  (params (AxisValue :type Float%20%28single-precision%29))
  (bind _returnvalue (Pawn|GetControlRotation :!class /Script/Engine.Pawn))
  ;[1 1 1] Left/Right Movement.
  (Pawn|Input|AddMovementInput (Math|Vector|GetRightVector (Math|Rotator|MakeRotator (.roll _returnvalue) 0.0 (.yaw _returnvalue))) AxisValue false))

(event Input|KeyboardEvents|DebugKeyH
  (params (Key :type Key%20Structure :default "None") (ActionValue :type Input%20Action%20Value%20Structure))
  ;[1 1 1] TEMP | Manual Healing for Testing
  (:Pressed
    (CallFunction|Heal 1e+01)))

(event Input|MouseEvents|LeftMouseButton
  (params (Key :type Key%20Structure :default "None"))
  ;[1 1 1] TEMP | Manual clicking for damage to enemies for testing purposes.
)

(fn ConstructionScript)

(fn AddXp
  (params (CurrentXP :type Float%20%28double-precision%29))
  (bind _output_get (Variables|Stats|SetCurrentXP (+ CurrentXP (+ (* (Variables|Stats|GetCurrentXP) (Variables|Passives|GetXPPercentIncrease)) (Variables|Stats|GetCurrentXP)))))
  (if (>= _output_get (Variables|Stats|GetXPtoLevel))
    (CallFunction|LevelUpMenu)
    ;[1 1 1] Controlls the XP increase requirement per level
    (Math|Integer|IncrementInt (Variables|Stats|GetPlayerLevel)
      (:%20%20
        (Variables|Stats|SetCurrentXP (- (Variables|Stats|GetCurrentXP) (Variables|Stats|GetXPtoLevel)))
        (Variables|Stats|SetXPtoLevel (* (Variables|Stats|GetXPtoLevel) 1.2))
        (return (Variables|Stats|GetPlayerLevel))))))

(fn LevelUpMenu
  ;[1 1 1] Pauses game upon leveling up and adds level up menu to screen
  (Game|SetGamePaused true)
  (bind _returnvalue (UserInterface|CreateWidget "/Game/UI/WBP_LevelUp.WBP_LevelUp_C"))
  (UserInterface|Viewport|AddtoViewport _returnvalue 0))

(fn IncreaseMaxHP
  (Variables|Stats|SetMaxHealth (+ (* (Variables|Stats|GetMaxHealth) 0.15) (Variables|Stats|GetMaxHealth)))
  (Math|Integer|IncrementInt (Variables|PassiveLevels|GetMaxHPLevel)
    (:%20%20
      (return))))

(fn IncreaseFireRate
  (Variables|Passives|SetFireRate (- (Variables|Passives|GetFireRate) 1.0))
  (Math|Integer|IncrementInt (Variables|PassiveLevels|GetFireRateLevel)))

(fn IncreaseXPGain
  ;[1 0.8371 0.1514] Currently increases XP gain by 10%. Needs to be refined.
  (Variables|Passives|SetXPPercentIncrease (+ (Variables|Passives|GetXPPercentIncrease) 0.1))
  (Math|Integer|IncrementInt (Variables|PassiveLevels|GetXPIncreaseLevel)))

(fn DamageEnemiesOnce
  (params (EnemyHits :type Array%20of%20Hit%20Result%20Structures) (Damage :type Float%20%28double-precision%29) (Instigator :type Controller%20Object%20Reference) (Causer :type Actor%20Object%20Reference))
  (bind _l_hitactors (Variables|Default|GetL_HitActors))
  (for _index (range 0 (Utilities|Array|LastIndex EnemyHits))
    (if (not (Utilities|Array|ContainsItem _l_hitactors (.HitActor (Collision|BreakHitResult (Utilities|Array|Get(acopy) EnemyHits _index)))))
      (Utilities|Array|Add _l_hitactors (.HitActor (Collision|BreakHitResult (Utilities|Array|Get(acopy) EnemyHits _index))))
      (Game|Damage|ApplyDamage (.HitActor (Collision|BreakHitResult (Utilities|Array|Get(acopy) EnemyHits _index))) (Variables|Default|GetDamage) (Variables|Default|GetInstigator_0) (Variables|Default|GetCauser)))))

(fn SetSelectedAbility
  (bind _abilitiestag (Variables|Default|GetAbilitiesTag))
  (bind _icon (Utilities|CheckAbilitySwitch)
    (:Stop
      (return))
    (:Proceed
      (if (GameplayTags|HasTag _abilitiestag "(TagName=\"PassiveSlot1\")" true)
        (if (GameplayTags|HasTag _abilitiestag "(TagName=\"PassiveSlot2\")" true)
          (if (GameplayTags|HasTag _abilitiestag "(TagName=\"PassiveSlot3\")" true)
            (return)
            (else
              (GameplayTags|AddGameplayTag _abilitiestag "(TagName=\"PassiveSlot3\")" :!class /Script/GameplayTags.BlueprintGameplayTagLibrary)
              (Class|BPIAbilities|SetPassive3(Message) self _icon "None")
              (return)))
          (else
            (GameplayTags|AddGameplayTag _abilitiestag "(TagName=\"PassiveSlot2\")" :!class /Script/GameplayTags.BlueprintGameplayTagLibrary)
            (Class|BPIAbilities|SetPassive2(Message) self _icon "None")
            (return)))
        (else
          (GameplayTags|AddGameplayTag _abilitiestag "(TagName=\"PassiveSlot1\")" :!class /Script/GameplayTags.BlueprintGameplayTagLibrary)
          (Class|BPIAbilities|SetPassive1(Message) self _icon "None")
          (return))))))

(fn GetAbility
  (return (Variables|Default|GetAssignedAbility)))

(fn GetAbilityComponent
  (return (Variables|Default|GetBPC_AbilitySystem)))

(fn GetAbilityTag
  (return (Variables|Default|GetAbilitiesTag)))

(fn GetMaxHPPassiveLvl
  (return (Variables|PassiveLevels|GetMaxHPLevel)))

(fn GetPassive1
  (return (Variables|PassiveLevels|GetPassiveIcon1) (Variables|PassiveLevels|GetPassiveName1)))

(fn GetPassive2
  (return (Variables|PassiveLevels|GetPassiveIcon2) (Variables|PassiveLevels|GetPassiveName2)))

(fn GetPassive3
  (return (Variables|PassiveLevels|GetPassiveIcon3) (Variables|PassiveLevels|GetPassiveName3)))

(fn GetPlayerCurrentHealth
  (return (Variables|Stats|GetCurrentHealth)))

(fn GetPlayerDeathStatus
  (return (Variables|Default|GetIsDead?)))

(fn GetPlayerLevel
  (return (Variables|Stats|GetPlayerLevel)))

(fn GetPlayerMaxHealth
  (return (Variables|Stats|GetMaxHealth)))

(fn GetPlayerXP
  (return (Variables|Stats|GetCurrentXP)))

(fn GetProjectileSpawner
  (return (Variables|Default|GetProjectileSpawnLocation)))

(fn GetXptoLevel
  (return (Variables|Stats|GetXPtoLevel)))

(fn Heal
  (params (HealAmount :type Float%20%28double-precision%29)))

(fn TakeDamage
  (params (DamgeInfo :type BPS%20Damage%20Info%20Structure)))