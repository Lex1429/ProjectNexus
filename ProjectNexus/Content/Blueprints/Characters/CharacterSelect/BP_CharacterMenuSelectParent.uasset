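; Parent Blueprint for a selectable character in the character select menu, with handlers that toggle custom depth rendering on hover.
; GetCharacterData looks up the class name, description, icon, color and Blueprint in DT_Classes.
; Click and BeginPlay events are empty.
; The logic that binds the cursor handlers, sets SkeletalRef, saves the selected class to the GameInstance and opens TestLevel is disconnected, so it never runs.
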(event OnClicked(SkeletalMesh)
  (params (TouchedComponent :type Primitive%20Component%20Object%20Reference) (ButtonPressed :type Key%20Structure :default "None")))

(event Custom|OnMouseClicked
  (params (TouchedActor :type Actor%20Object%20Reference) (ButtonPressed :type Key%20Structure :default "None")))

(event Custom|OnMouseHover
  (params (TouchedActor :type Actor%20Object%20Reference))
  (Rendering|SetRenderCustomDepth (Variables|Default|GetSkeletalRef) true))

(event Custom|OnMouseExit
  (params (TouchedActor :type Actor%20Object%20Reference))
  (Rendering|SetRenderCustomDepth (Variables|Default|GetSkeletalRef) false))

(event EventBeginPlay)

(fn ConstructionScript)

(fn GetCharacterData
  (bind _returnvalue (Utilities|GetDataTableRow "/Game/Blueprints/DataTables/DT_Classes.DT_Classes" (.RowName (Utilities|Struct|BreakDataTableRowHandle (Variables|Default|GetCharacterData))))
    (:then
      (return (.ClassName (Utilities|Struct|BreakBPS_Classes _returnvalue)) (.Description (Utilities|Struct|BreakBPS_Classes _returnvalue)) (.ClassIcon (Utilities|Struct|BreakBPS_Classes _returnvalue)) (.ClassBP (Utilities|Struct|BreakBPS_Classes _returnvalue)) (.IconColor (Utilities|Struct|BreakBPS_Classes _returnvalue))))))