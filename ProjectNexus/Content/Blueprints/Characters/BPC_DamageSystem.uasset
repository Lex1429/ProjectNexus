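; Actor component that manages a character's health, healing and death.
; TakeDamage passes each DamageInfo through a CanBeDamaged exec-branch gate that blocks dead or invincible owners, unless the hit ignores invincibility.
; Applied damage either marks death and fires OnDeath, or fires OnDamageResponse when the owner is interruptible or the hit forces an interrupt.
; Heal adds health clamped to MaxHealth, only while alive.
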(event EventBeginPlay)

(event EventTick
  (params (DeltaSeconds :type Float%20%28single-precision%29)))

(fn Heal
  (params (HealAmount :type Float%20%28double-precision%29))
  (if (not (Variables|Default|GetIsDead?))
    (bind _output_get (Variables|Default|SetCurrentHealth (Math|Float|Clamp(Float) (+ HealAmount (Variables|Default|GetCurrentHealth)) 0.0 (Variables|Default|GetMaxHealth))))
    (return _output_get)))

(fn TakeDamage
  (params (DamageInfo :type BPS%20Damage%20Info%20Structure))
  (bind (_amount _damagetype _damageresponse _shoulddamageinvincible _shouldforceinterrupt) (Utilities|Struct|BreakBPS_DamageInfo DamageInfo))
  (Utilities|CanbeDamaged? _shoulddamageinvincible
    (:DoDamage
      (bind _output_get (Variables|Default|SetCurrentHealth (- (Variables|Default|GetCurrentHealth) _amount)))
      (if (<= _output_get 0.0) ; If Actor's health is at or below zero, they are set to a dead state
        (Variables|Default|SetIsDead? true)
        (Default|CallOnDeath)
        (return true)
        (elif (or (Variables|Default|GetIsInterruptible?) _shouldforceinterrupt)
          (Default|CallOnDamageResponse _damageresponse)
          (return true))))
    (:NoDamage
      (return false))))