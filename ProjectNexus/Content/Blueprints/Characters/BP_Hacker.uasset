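; BP_Hacker is a character Blueprint that emits a recurring area-of-effect electric field from BeginPlay.
; ElectricField runs immediately and sets a looping FireRate timer on itself, each pulse spawning a BP_AoE_Explosion attached to the mesh's AOESocket.
; It binds the explosion's overlap event to DamageEnemy, then triggers it.
; DamageEnemy sends overlapped actors a fixed damage message that forces an interrupt.
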(event Custom|ElectricField
  (Utilities|Time|SetTimerbyFunctionName 0 "ElectricField" (Variables|Default|GetFireRate) true)
  (bind _returnvalue (Game|SpawnActorfromClass "/Game/Blueprints/Melee/BP_AoE_Explosion.BP_AoE_Explosion_C" (Transformation|GetActorTransform) "Undefined" "MultiplyWithRoot" 0 true false false 0))
  (Transformation|AttachComponentToComponent _returnvalue (Variables|Character|GetMesh) "AOESocket" "SnapToTarget" "SnapToTarget" "SnapToTarget" true)
  (EventDispatchers|BindEventtoOnAOEOverlapActor _returnvalue (delegate Custom|DamageEnemy))
  (Default|Trigger _returnvalue))

(event Custom|DamageEnemy
  (params (Actor :type Actor%20Object%20Reference))
  (Class|BPIPlayerStats|TakeDamage(Message) Actor (Utilities|Struct|MakeBPS_DamageInfo 5e+01 "NewEnumerator3" "NewEnumerator2" false true)))

(event EventBeginPlay
  (CallFunction|ElectricField))

(fn ConstructionScript
  (|CallParentFunction))