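; BP_Computer is an interactable computer actor that shows a widget while something overlaps its Sphere.
; Interact calls DrainProgressBar, which runs only while ShouldDrain is set and lowers ProgressBarAmount in small clamped steps.
; The drain re-calls itself after a short Delay instead of using Tick, and clears ShouldDrain when the amount reaches zero.
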(event OnComponentBeginOverlap(Sphere)
  (params (OverlappedComponent :type Primitive%20Component%20Object%20Reference) (OtherActor :type Actor%20Object%20Reference) (OtherComp :type Primitive%20Component%20Object%20Reference) (OtherBodyIndex :type Integer) (bFromSweep :type Boolean) (SweepResult :type Hit%20Result%20Structure%20%28by%20ref%29))
  (Rendering|SetVisibility (Variables|Default|GetWidget) true false))

(event OnComponentEndOverlap(Sphere)
  (params (OverlappedComponent :type Primitive%20Component%20Object%20Reference) (OtherActor :type Actor%20Object%20Reference) (OtherComp :type Primitive%20Component%20Object%20Reference) (OtherBodyIndex :type Integer))
  (Rendering|SetVisibility (Variables|Default|GetWidget) false false))

(event Custom|DrainProgressBar
  (if (Variables|Default|GetShouldDrain?)
    (bind _output_get (Variables|Default|SetProgressBarAmount (Math|Float|Clamp(Float) (- (Variables|Default|GetProgressBarAmount) 0.5) 0.0 (Variables|Default|GetProgressBarMax))))
    (if (== _output_get 0.0)
      (Variables|Default|SetShouldDrain? false)
      (else
        (Utilities|FlowControl|Delay 0.01)
        (CallFunction|DrainProgressBar)))))

(event EventBeginPlay
  (|CallParentFunction) ; This node is disabled and will not be called.\nDrag off pins to build functionality.
)

(event Collision|EventActorBeginOverlap
  (params (OtherActor :type Actor%20Object%20Reference))
  (|CallParentFunction OtherActor) ; This node is disabled and will not be called.\nDrag off pins to build functionality.
)

(event EventTick
  (params (DeltaSeconds :type Float%20%28single-precision%29))
  (|CallParentFunction DeltaSeconds) ; This node is disabled and will not be called.\nDrag off pins to build functionality.
)

(event EventInteract
  (CallFunction|DrainProgressBar))

(fn ConstructionScript
  (|CallParentFunction))