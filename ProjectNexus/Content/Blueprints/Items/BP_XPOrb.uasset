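; BP_XPOrb is an experience orb item that grants XP to the player on overlap.
; Its Trigger component checks overlapping actors for the Player tag, casts to BP_BaseCharacterClass and calls OrbXPIncrease with the SmallXP amount.
; The graph does not destroy the orb afterwards.
; Its player stat, Heal and TakeDamage functions are stubs returning default values.
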(event OnComponentBeginOverlap(Trigger)
  (params (OverlappedComponent :type Primitive%20Component%20Object%20Reference) (OtherActor :type Actor%20Object%20Reference) (OtherComp :type Primitive%20Component%20Object%20Reference) (OtherBodyIndex :type Integer) (bFromSweep :type Boolean) (SweepResult :type Hit%20Result%20Structure%20%28by%20ref%29))
  (if (Actor|ActorHasTag OtherActor "Player")
    (bind _asbp_base_character_class (Utilities|Casting|CastToBP_BaseCharacterClass OtherActor))
    (Default|OrbXPIncrease _asbp_base_character_class (Variables|Default|GetSmallXP))))

(event EventBeginPlay
  (|CallParentFunction) ; This node is disabled and will not be called.\nDrag off pins to build functionality.
)

(event Collision|EventActorBeginOverlap
  (params (OtherActor :type Actor%20Object%20Reference))
  (|CallParentFunction OtherActor) ; This node is disabled and will not be called.\nDrag off pins to build functionality.
)

(event EventTick
  (params (DeltaSeconds :type Float%20%28single-precision%29))
  (|CallParentFunction DeltaSeconds) ; This node is disabled and will not be called.\nDrag off pins to build functionality.
)

(fn ConstructionScript
  (|CallParentFunction))

(fn GetPlayerCurrentHealth
  (return 0.0))

(fn GetPlayerDeathStatus
  (return false))

(fn GetPlayerLevel
  (return 0))

(fn GetPlayerMaxHealth
  (return 0.0))

(fn GetPlayerXP
  (return 0.0))

(fn GetXptoLevel
  (return 0.0))

(fn Heal
  (params (HealAmount :type Float%20%28double-precision%29))
  (return 0.0))

(fn TakeDamage
  (params (DaamgeInfo :type BPS%20Damage%20Info%20Structure))
  (return false))